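; BP_Button is a pressable mechanism button that works only while its Usable flag is set.
; Pressing it sends an Activate message to Mechanism with NextButton, prints the result, disables the button and calls the UseButton dispatcher.
; ActivateButton re-enables it, with Cube2 switching between pulsing and plain hex-tile materials to show the state.
; The construction script applies the matching material from the initial Usable value.
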(event `PressButton`
  ;[1 1 1] Взамиодействие кнопки и предмета
  (if (`self.Usable`)
    (bind _success (message `/Game/Content/BP/Interface/BPI_Activation.Activate` (`self.Mechanism`) (`self.NextButton`)))
    (`KismetSystemLibrary.PrintString` (`KismetStringLibrary.Conv_BoolToString` _success))
    (set `self.Usable` false)
    (`self.UseButton`)
    (`PrimitiveComponent.SetMaterial` (`self.Cube2`) 0 "/Game/StarterContent/Materials/M_Tech_Hex_Tile.M_Tech_Hex_Tile")
    (else
      (`KismetSystemLibrary.PrintString` "This button cannot be used"))))

(event `ActivateButton`
  ;[1 1 1] Активируем кнопку
  (set `self.Usable` true)
  (`PrimitiveComponent.SetMaterial` (`self.Cube2`) 0 "/Game/StarterContent/Materials/M_Tech_Hex_Tile_Pulse.M_Tech_Hex_Tile_Pulse"))

(fn `UserConstructionScript`
  (if (`self.Usable`)
    (`PrimitiveComponent.SetMaterial` (`self.Cube2`) 0 "/Game/StarterContent/Materials/M_Tech_Hex_Tile_Pulse.M_Tech_Hex_Tile_Pulse")
    (else
      (`PrimitiveComponent.SetMaterial` (`self.Cube2`) 0 "/Game/StarterContent/Materials/M_Tech_Hex_Tile.M_Tech_Hex_Tile"))))