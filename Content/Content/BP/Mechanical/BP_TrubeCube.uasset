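; BP_TrubeCube is a mechanical tube that spawns a BP_Cube when activated.
; Activate stores the passed NextButton and, unless the tube is busy, starts the AnimOpen timeline, which pitches the Cap.
; A timeline event track spawns the cube at the actor's transform.
; On finish, the timeline clears the Opened busy flag and calls ActivateButton on NextButton.
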(event `self.ReceiveBeginPlay`)

(event `OpenTrube`
  (bind _cap (`self.Cap`))
  (bind (_returnvalue_roll _returnvalue_pitch _returnvalue_yaw) (`KismetMathLibrary.BreakRotator` (`SceneComponent.K2_GetComponentRotation` _cap)))
  ;[1 1 1] Анимация открытия трубы
  (bind (_direction _yrotation) (`Timeline|AnimOpen` :!via `PlayFromStart`)
    (:`Update`
      (`SceneComponent.K2_SetWorldRotation` _cap (`KismetMathLibrary.MakeRotator` _returnvalue_roll _yrotation _returnvalue_yaw) false false))
    (:`Finished`
      (set `self.Opened` false)
      (`/Game/Content/BP/Mechanical/BP_Button.ActivateButton` (`self.NextButton`)))
    (:`SpawnCube`
      (`|SpawnActorFromClass` "/Game/Content/BP/Mechanical/BP_Cube.BP_Cube_C" (`self.GetTransform`) "Undefined" "OverrideRootScale" null null))))

(fn `Activate`
  (params (NextButton :type "/Game/Content/BP/Mechanical/BP_Button Object Reference"))
  (returns (Success :type Boolean) (Wait :type "Float (double-precision)"))
  (set `self.NextButton` NextButton)
  (if (`self.Opened`)
    (`KismetSystemLibrary.PrintString` "Whait. The cube is spawning")
    (else
      (set `self.Opened` true)
      (`self.OpenTrube`)))
  (return true 0.0))

(fn `UserConstructionScript`)