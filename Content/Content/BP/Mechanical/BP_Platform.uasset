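; BP_Platform is a mechanical moving platform (a minecart, per the comments) that shuttles along world Y when activated.
; Activate stores a NextButton and calls ChangeMove, which flips Right and plays or reverses the Way timeline that sets the actor's Y.
; When the forward move finishes, it activates NextButton and binds to its use event, which triggers ChangeMove again after a short delay to send the platform back.
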(event `ChangeMove`
  (bind (_returnvalue_x _returnvalue_y _returnvalue_z) (`KismetMathLibrary.BreakVector` (`self.K2_GetActorLocation`)))
  (bind _nextbutton (`self.NextButton`))
  ;[1 1 1] Анимация передвижения вагонетки
  (if (`self.Right`)
    (set `self.Right` false)
    (bind (_direction _y) (`Timeline|Way` :!label _label)
      (:`Update`
        (`self.K2_SetActorLocation` (`KismetMathLibrary.MakeVector` _returnvalue_x _y _returnvalue_z)))
      (:`Finished`
        (if (not (`self.Right`))
          (`/Game/Content/BP/Mechanical/BP_Button.ActivateButton` _nextbutton)
          ;[1 1 1] Ждем активации следующей кнопки, для того, чтобы вернуть платформу на место
          (add `/Game/Content/BP/Mechanical/BP_Button.UseButton` _nextbutton (delegate `ToggleNext`)))))
    (else
      (set `self.Right` true)
      (goto _label :!via `Reverse`))))

(event `ToggleNext`
  ;[1 1 1] Ждем активации следующей кнопки, для того, чтобы вернуть платформу на место
  (`KismetSystemLibrary.Delay` 3.0)
  (`self.ChangeMove`))

(fn `Activate`
  (params (NextButton :type "/Game/Content/BP/Mechanical/BP_Button Object Reference"))
  (returns (Success :type Boolean) (Wait :type "Float (double-precision)"))
  (set `self.NextButton` NextButton)
  (`self.ChangeMove`)
  (return true 0.0))

(fn `UserConstructionScript`)