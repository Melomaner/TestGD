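; Crane mechanism that, once activated, plays a timeline animation and carries a BP_Cube with a toggleable magnet.
; The timeline moves the Mechanim component and fires Magnite events that toggle the magnet and the held cube's physics.
; A box overlap captures the cube, which Tick interpolates toward Point with growing strength while the magnet is on.
; When finished, it resets and activates the button passed into Activate, chaining mechanisms.
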(event `StartMashinim`
  ;[1 1 1] Анимация передвижения крана
  (bind (_direction _vectormechanim) (`Timeline|UseCrane` :!via `PlayFromStart`)
    (:`Update`
      (`SceneComponent.K2_SetRelativeLocation` (`self.Mechanim`) _vectormechanim false false))
    (:`Finished`
      (set `self.Usable` false)
      ;[1 1 1] Обнуляем параметры магнита
      (set `self.MagnitItem` null)
      (set `self.DeltaTime` 1.0)
      (`/Game/Content/BP/Mechanical/BP_Button.ActivateButton` (`self.NextButton`)))
    (:`Magnite`
      (`self.Magnite`))))

(event `self.ReceiveTick`
  (params (DeltaSeconds :type "Float (single-precision)"))
  (bind _returnvalue (`GameplayStatics.GetWorldDeltaSeconds`))
  (bind _deltatime (`self.DeltaTime`))
  (bind _magnititem (`self.MagnitItem`))
  ;[1 1 1] Работа магнита у крана
  (if (`self.UseMagnite?`)
    (set `self.DeltaTime` (+ _deltatime (* _returnvalue 10.0)))
    (`/Engine/EditorBlueprintResources/StandardMacros.IsValid` _magnititem
      (:`Is Valid`
        (`self.K2_SetActorLocation` _magnititem (`KismetMathLibrary.VInterpTo` (`self.K2_GetActorLocation` _magnititem) (`SceneComponent.K2_GetComponentLocation` (`self.Point`)) _deltatime _returnvalue) false false)))))

(event `self.Box.OnComponentBeginOverlap`
  (params (OverlappedComponent :type "PrimitiveComponent Object Reference") (OtherActor :type "Actor Object Reference") (OtherComp :type "PrimitiveComponent Object Reference") (OtherBodyIndex :type Integer) (bFromSweep :type Boolean) (SweepResult :type "HitResult Structure (by ref)"))
  ;[1 1 1] Запоминаем примагниченный предмет
  (`/Engine/EditorBlueprintResources/StandardMacros.IsValid` (`self.MagnitItem`)
    (:`Is Not Valid`
      (bind _asbp_cube (cast `/Game/Content/BP/Mechanical/BP_Cube` OtherActor))
      (set `self.MagnitItem` _asbp_cube))))

(fn `Activate`
  (params (NextButton :type "/Game/Content/BP/Mechanical/BP_Button Object Reference"))
  (returns (Success :type Boolean) (Wait :type "Float (double-precision)"))
  (set `self.NextButton` NextButton)
  (if (`self.Usable`)
    (`KismetSystemLibrary.PrintString` "Whait. mashinim Working")
    (else
      (set `self.Usable` true)
      (`self.StartMashinim`)))
  (return true 0.0))

(fn `Magnite`
  (bind _magnititem (`self.MagnitItem`))
  (bind _magnititem_2 (`self.MagnitItem`))
  (if (`self.UseMagnite?`)
    (set `self.UseMagnite?` false)
    (`/Engine/EditorBlueprintResources/StandardMacros.IsValid` _magnititem_2
      (:`Is Valid`
        (`PrimitiveComponent.SetSimulatePhysics` (`/Game/Content/BP/Mechanical/BP_Cube.Cube` _magnititem_2) true)))
    (else
      (set `self.UseMagnite?` true)
      (`/Engine/EditorBlueprintResources/StandardMacros.IsValid` _magnititem
        (:`Is Valid`
          (`PrimitiveComponent.SetSimulatePhysics` (`/Game/Content/BP/Mechanical/BP_Cube.Cube` _magnititem) false))))))

(fn `UserConstructionScript`)