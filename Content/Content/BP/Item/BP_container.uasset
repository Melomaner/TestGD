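; BP_container is a locked container that opens when the player's inventory holds the key.
; Its Open event calls FindItem on the player pawn's BC_Inventory and, on success, plays the OpenBox timeline to slide W1 along relative Y.
; ContainerOpen is set when the timeline finishes and blocks later openings.
; Printed messages report success, a missing key or an already open container, while a missing inventory component fails silently.
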(event `Open`
  (bind _w1 (`self.w1`))
  (bind _returnvalue (`self.GetComponentByClass` (`GameplayStatics.GetPlayerPawn` 0) "/Game/Content/BP/Component/BC_Inventory.BC_Inventory_C"))
  (bind (_relativelocation_x _relativelocation_y _relativelocation_z) (`KismetMathLibrary.BreakVector` (`SceneComponent.RelativeLocation` _w1)))
  (if (`self.ContainerOpen`)
    (`KismetSystemLibrary.PrintString` "The container has already been opened earlier \n")
    (else
      (`/Engine/EditorBlueprintResources/StandardMacros.IsValid` _returnvalue
        (:`Is Valid`
          (bind _have (`/Game/Content/BP/Component/BC_Inventory.FindItem` _returnvalue))
          (if _have
            (bind (_direction _open) (`Timeline|Open box`)
              (:`Update`
                (`SceneComponent.K2_SetRelativeLocation` _w1 (`KismetMathLibrary.MakeVector` _relativelocation_x _open _relativelocation_z) false false))
              (:`Finished`
                (`KismetSystemLibrary.PrintString` "You have opened a container")
                (set `self.ContainerOpen` true)))
            (else
              (`KismetSystemLibrary.PrintString` "You do not have a key to open the container"))))))))

(fn `UserConstructionScript`)